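; Swingable rope actor that a player can grab and push back and forth through a physics-driven cable end.
; Box overlap passes the rope to the player via interface messages; leaving clears it and starts a regrab cooldown.
; AddSwingingForce applies scaled impulses while the end hangs low enough, with a large one-time kick per grab.
; Linear damping switches with input and height to sustain or settle the swing.
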(event `self.Box.OnComponentBeginOverlap`
  (params (OverlappedComponent :type "PrimitiveComponent Object Reference") (OtherActor :type "Actor Object Reference") (OtherComp :type "PrimitiveComponent Object Reference") (OtherBodyIndex :type Integer) (bFromSweep :type Boolean) (SweepResult :type "HitResult Structure (by ref)"))
  (if (`self.IsGrabable`)
    (bind (_yesorno _referance) (message `/Game/SwingngSystem/RopetoPlayer_BPI.IsPlayerRope` OtherActor))
    (if (and _yesorno (`KismetSystemLibrary.IsValid` _referance))
      (message `/Game/SwingngSystem/RopetoPlayer_BPI.RopeSave` _referance self)
      (set `self.IsGrabable` false))))

(event `AddSwingingForce`
  (params (SwingForce :type "Vector Structure") (Scale :type "Float (double-precision)"))
  (bind (_returnvalue_x _returnvalue_y _returnvalue_z) (`KismetMathLibrary.BreakVector` (`self.K2_GetActorLocation`)))
  (bind _cableend (`self.CableEnd`))
  (bind _returnvalue (* (* SwingForce 300.0) Scale))
  (bind (_returnvalue_x_2 _returnvalue_y_2 _returnvalue_z_2) (`KismetMathLibrary.BreakVector` (`SceneComponent.K2_GetComponentLocation` (`self.CableEnd`))))
  (if (> (- _returnvalue_z _returnvalue_z_2) 370.0)
    (if (== Scale 0.0)
      (`PrimitiveComponent.SetLinearDamping` _cableend 0.7)
      (else
        (`PrimitiveComponent.SetLinearDamping` _cableend 0.01)))
    (`PrimitiveComponent.AddImpulse` _cableend _returnvalue "None" false)
    (`/Engine/EditorBlueprintResources/StandardMacros.DoOnce` false :!label _label
      (:`Completed`
        (`PrimitiveComponent.AddImpulse` _cableend (* _returnvalue 200.0) "None" false)))
    (else
      (`PrimitiveComponent.SetLinearDamping` _cableend 1.0))))

(event `self.Box.OnComponentEndOverlap`
  (params (OverlappedComponent :type "PrimitiveComponent Object Reference") (OtherActor :type "Actor Object Reference") (OtherComp :type "PrimitiveComponent Object Reference") (OtherBodyIndex :type Integer))
  (set `self.IsGrabable` false)
  (`PrimitiveComponent.SetLinearDamping` (`self.CableEnd`) 0.7)
  (`KismetSystemLibrary.K2_SetTimerDelegate` (delegate `SetGrabable`) 2.0)
  (message `/Game/SwingngSystem/RopetoPlayer_BPI.RopeSave` OtherActor null)
  (goto _label :!via `Reset`))

(event `SetGrabable`
  (set `self.IsGrabable` true))

(fn `SetCableEndMassInKG`)

(fn `UserConstructionScript`)