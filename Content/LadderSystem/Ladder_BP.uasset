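; Climbable ladder actor that builds itself to a configurable Height and registers itself with player characters that touch it.
; InitLadder, run at construction and BeginPlay, positions the top, stretches both side bars and the main collider to fit, and adds instanced-mesh rungs every CrossbarGap.
; The main and lower colliders query overlapping actors through interface-style messages and hand qualifying players a reference to the ladder.
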(event `self.ReceiveBeginPlay`
  (`self.Init_Ladder`))

(event `Init_Ladder`
  (bind _temp_height (`self.temp_height`))
  (bind (_relativelocation_x _relativelocation_y _relativelocation_z) (`KismetMathLibrary.BreakVector` (`SceneComponent.RelativeLocation` (`self.LadderTop`))))
  (`SceneComponent.K2_SetRelativeLocation` (`self.LadderTop`) (`KismetMathLibrary.MakeVector` 0.0 0.0 (`self.height`)) false false)
  (`self.Adjust Side Bar` (`self.Ladder_L`))
  (`self.Adjust Side Bar` (`self.Ladder_R`))
  (`self.Adjust Side Bar` (`self.LadderCollider`))
  (set `self.temp_height` 0.0)
  (while (< _temp_height _relativelocation_z)
    (`InstancedStaticMeshComponent.AddInstance` (`self.ism_Crossbar`) (`KismetMathLibrary.MakeTransform` (`KismetMathLibrary.MakeVector` 0.0 0.0 _temp_height) (struct) (0.11 0.8 0.1)))
    (set `self.temp_height` (+ _temp_height (`self.Crossbar_gap`)))))

(event `self.LadderCollider.OnComponentBeginOverlap`
  (params (OverlappedComponent :type "PrimitiveComponent Object Reference") (OtherActor :type "Actor Object Reference") (OtherComp :type "PrimitiveComponent Object Reference") (OtherBodyIndex :type Integer) (bFromSweep :type Boolean) (SweepResult :type "HitResult Structure (by ref)"))
  (bind (_yesorno _referance) (message `/Game/SwingngSystem/RopetoPlayer_BPI.IsPlayerRope` OtherActor))
  (if _yesorno
    (bind _output_get (set `self.CharRef` _referance))
    (message `/Game/LadderSystem/Ladder_BPI.SetLadder` _output_get self)))

(event `self.LadderDownColider.OnComponentBeginOverlap`
  (params (OverlappedComponent :type "PrimitiveComponent Object Reference") (OtherActor :type "Actor Object Reference") (OtherComp :type "PrimitiveComponent Object Reference") (OtherBodyIndex :type Integer) (bFromSweep :type Boolean) (SweepResult :type "HitResult Structure (by ref)"))
  (bind (_yesorno _referance) (message `/Game/SwingngSystem/RopetoPlayer_BPI.IsPlayerRope` OtherActor))
  (if _yesorno
    (bind _output_get (set `self.CharRef` _referance))
    (message `/Game/LadderSystem/Ladder_BPI.SetLadder` _output_get self)))

(fn `UserConstructionScript`
  (`self.Init_Ladder`))