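; Pushable actor that, when a non-jumping player interacts, teleports them to a push spot and starts pushing through their PushComponent.
; Push spots are relative transforms, shown as arrows by the construction script and searched by squared 2D distance within PushRange, stopping at the first accepted one.
; Capsule and line traces validate standing room, walkable floor and no blocking wall, with debug drawing and printed failure reasons.
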(event `/Game/InteractInterface/InteractInterface_BPI.OnInteracted`
  (params (Player :type "/Game/ThirdPersonBP/Blueprints/ThirdPersonCharacter Object Reference"))
  (if (not (`/Game/ThirdPersonBP/Blueprints/ThirdPersonCharacter.IsJumping` Player))
    (`self.Handle Interaction` Player)))

(fn `FindClosestPushTransformIndex`
  (params (CharLocation :type "Vector2D Structure") (PushRange :type "Float (double-precision)"))
  (locals (CurrentIndex :type Integer) (CurrentDistanceSq :type "Float (double-precision)" :default 0.0) (ClosestDistanceSq :type "Float (double-precision)" :default 100000.0) (ClosestTransformIndex :type Integer))
  (bind _pushtransforms (`self.PushTransforms`))
  (bind _currentindex (`local.CurrentIndex`))
  (bind _output_get (set `local.CurrentDistanceSq` (`KismetMathLibrary.DistanceSquared2D` (`KismetMathLibrary.Conv_VectorToVector2D` (`KismetMathLibrary.TransformLocation` (`self.GetTransform`) (.location (`|GetArrayItem` _pushtransforms _currentindex)))) (`local.CharLocation`)) :!label _label))
  (if (< _output_get (`KismetMathLibrary.Square` (`local.PushRange`)))
    (if (or (< (`local.CurrentDistanceSq`) (`local.ClosestDistanceSq`)) (< (`local.ClosestTransformIndex`) 0))
      (set `self.BestIndex` (`local.CurrentIndex`))
      (set `local.ClosestDistanceSq` (`local.CurrentDistanceSq`))
      (else
        (`/Engine/EditorBlueprintResources/StandardMacros.IncrementInt` _currentindex :!label _label_2
          (:`  `
            (if (< _currentindex (`KismetArrayLibrary.Array_Length` _pushtransforms))
              (goto _label)
              (else
                (return)))))))
    (else
      (goto _label_2))))

(fn `Handle Interaction`
  (params (Char :type "Character Object Reference"))
  (locals (PushComponent :type "/Game/Pushable/PushComponent Object Reference") (CharNewTransform :type "Transform Structure"))
  (bind _charnewtransform_location (`KismetMathLibrary.BreakTransform` (`local.CharNewTransform`)))
  (bind _bestindex (`self.BestIndex`))
  (bind _charnewtransform_location_2 (`KismetMathLibrary.BreakTransform` (`local.CharNewTransform`)))
  (bind _capsulecomponent (`Character.CapsuleComponent` (`local.Char`)))
  (bind (_returnvalue_location _returnvalue_rotation) (`KismetMathLibrary.BreakTransform` (`KismetMathLibrary.ComposeTransforms` (`|GetArrayItem` (`self.PushTransforms`) _bestindex) (`self.GetTransform`))))
  (`/Engine/EditorBlueprintResources/StandardMacros.IsValid` Char
    (:`Is Valid`
      (bind _output_get (set `local.PushComponent` (`self.GetComponentByClass` Char "/Game/Pushable/PushComponent.PushComponent_C")))
      (`/Engine/EditorBlueprintResources/StandardMacros.IsValid` _output_get
        (:`Is Valid`
          (`self.FindClosestPushTransformIndex` (`KismetMathLibrary.Conv_VectorToVector2D` (`self.K2_GetActorLocation` (`local.Char`))) (`/Game/Pushable/PushComponent.PushRange` (`local.PushComponent`)))
          (if (>= _bestindex 0)
            (bind _output_get_2 (set `local.CharNewTransform` (`KismetMathLibrary.MakeTransform` (+ _returnvalue_location (`KismetMathLibrary.MakeVector` 0.0 0.0 (`CapsuleComponent.GetScaledCapsuleHalfHeight` (`Character.CapsuleComponent` (`local.Char`))))) _returnvalue_rotation (.scale (`self.GetTransform` (`local.Char`))))))
            (`KismetSystemLibrary.DrawDebugSphere` (.location _output_get_2) 20.0 12 (struct :`R` 1.0 :`G` 0.027873 :`A` 1.0) 2.0 1.0)
            (bind _outhit (`KismetSystemLibrary.CapsuleTraceSingle` :`Start` (+ _charnewtransform_location_2 (0.0 0.0 70.0)) :`End` (- _charnewtransform_location_2 (0.0 0.0 100.0)) :`Radius` (`CapsuleComponent.GetScaledCapsuleRadius` _capsulecomponent) :`HalfHeight` (`CapsuleComponent.GetScaledCapsuleHalfHeight` _capsulecomponent) :`TraceChannel` "TraceTypeQuery1" :`DrawDebugType` "ForDuration" :`DrawTime` 2.0))
            (bind (_bblockinghit _binitialoverlap _time _distance _location _impactpoint _normal _impactnormal) (`GameplayStatics.BreakHitResult` _outhit))
            (if (not _binitialoverlap)
              (if (< (`CharacterMovementComponent.K2_GetWalkableFloorZ` (`Character.CharacterMovement` (`local.Char`))) (.z _impactnormal))
                (bind (_outhit_2 _returnvalue) (`KismetSystemLibrary.LineTraceSingle` (`self.K2_GetActorLocation`) _charnewtransform_location "TraceTypeQuery1" false (`|MakeArray` (`local.Char`) :!type "Actor Object Reference") "ForDuration" true (struct :`R` 1.0 :`A` 1.0) (struct :`G` 1.0 :`A` 1.0) 2.0))
                (if (not _returnvalue)
                  (`self.K2_SetActorTransform` (`local.Char`) (`local.CharNewTransform`) false true)
                  (`/Game/Pushable/PushComponent.BeginPush` (`local.PushComponent`) self)
                  (else
                    (`self.PushFailedIntro` "Wall in between char or object")))
                (else
                  (`self.PushFailedIntro` "Floor Not walkable")))
              (else
                (`self.PushFailedIntro` "No room to stand")))
            (else
              (`self.PushFailedIntro` "NOT Find Push Transform"))))
        (:`Is Not Valid`
          (`self.PushFailedIntro` "Char does NOT have Push Component"))))
    (:`Is Not Valid`
      (`self.PushFailedIntro` "Char is NOT valid"))))

(fn `UserConstructionScript`
  (for _array_element (`self.PushTransforms`)
    (`AddComponent|NODE_AddArrowComponent-0` :`RelativeTransform` _array_element)))